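; Test NPC that patrols, chases the player on sight and ends the game on reaching them.
; Patrolling loops AIMoveTo through four PatrolLocation entries at walking speed, with random pauses.
; A player overlap with VisionRange starts a faster chase with spotted audio; success shows the game-over widget, sound and cursor.
; GetKilled only sets StopOnOverlap, a flag fed into the chase move.
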(event OnComponentBeginOverlap(VisionRange)
  (params (OverlappedComponent :type Primitive%20Component%20Object%20Reference) (OtherActor :type Actor%20Object%20Reference) (OtherComp :type Primitive%20Component%20Object%20Reference) (OtherBodyIndex :type Integer) (bFromSweep :type Boolean) (SweepResult :type Hit%20Result%20Structure%20%28by%20ref%29))
  ;[1 0.3394 0] Chasing
  (Utilities|Casting|CastToTopDOwnCharacter_BP OtherActor)
  (CallFunction|Chasing))

(event Custom|Patrolling
  ;[0 0.1244 1] Patrolling
  (Variables|/Script/Engine.CharacterMovementComponent|SetMaxWalkSpeed (Variables|Character|GetCharacterMovement) 1.5e+02)
  (AI|AIMoveTo self (Utilities|Array|Get(acopy) (Variables|Default|GetPatrolLocation) (Variables|Default|GetLocations)) 0 5.0 false
    (:OnSuccess
      (Utilities|FlowControl|Delay (Math|Random|RandomFloatinRange 3.0 6.0))
      (CallFunction|Patrolling)
      (Math|Integer|IncrementInt (Variables|Default|GetLocations)
        (:%20%20
          (if (== (Variables|Default|GetLocations) 4)
            (Variables|Default|SetLocations 0)))))))

(event Custom|Chasing
  (bind _returnvalue (Game|GetPlayerController 0))
  ;[1 0.3394 0] Chasing
  (Variables|/Script/Engine.CharacterMovementComponent|SetMaxWalkSpeed (Variables|Character|GetCharacterMovement) 3e+02)
  (AI|AIMoveTo self "0, 0, 0" (Game|GetPlayerCharacter 0) 2.0 (Variables|Default|GetStop%20on%20Overlap)
    (:then
      ;;[1 0.8685 0] Sound
      (bind _returnvalue_2 (AddComponent|AddAudioComponent false))
      (Variables|Default|SetIsplaingSpotted _returnvalue_2))
    (:OnSuccess
      (Audio|Components|Audio|Stop (Variables|Default|GetIsplaingSpotted))
      (bind _returnvalue_3 (UserInterface|CreateWidget "/Game/Widgets/GameOverWidget_BP.GameOverWidget_BP_C"))
      (Audio|PlaySound2D "/Game/Sound/SFX/GameOver.GameOver" 1.0 1.0 0.0 0 0)
      (UserInterface|Viewport|AddtoViewport _returnvalue_3 0)
      (Input|SetInputModeUIOnly _returnvalue 0 "DoNotLock" false)
      (Variables|/Script/Engine.PlayerController|SetbShowMouseCursor _returnvalue true))
    (:OnFail
      (Audio|Components|Audio|Stop (Variables|Default|GetIsplaingSpotted)))))

(event Custom|GetKilled
  (if true
    (Variables|Default|SetStop%20on%20Overlap true)))

(event EventBeginPlay
  ;[0.7816 1 0] Begin
  (CallFunction|Patrolling))

(fn ConstructionScript)