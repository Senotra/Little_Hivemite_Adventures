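; Interactable distraction object that plays a distraction sound when triggered by the player.
; Entering the prompt collision as the top-down character shows text and a prompt and enables E; hovering the click collision also shows the text.
; E or a click from any distance runs the same trigger, which hides the prompt and locks reuse for a short delay.
; The prompt then reappears without rechecking overlap; no AI is notified here.
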(event OnClicked(ClickCollision)
  (params (TouchedComponent :type Primitive%20Component%20Object%20Reference) (ButtonPressed :type Key%20Structure :default "None"))
  ;[0 0.2976 1] Triggered
  (if (Variables|Default|GetDistractionActive)
    (Development|PrintString "Active")
    (else
      (Variables|Default|SetDistractionActive true)
      (Rendering|SetVisibility (Variables|Default|GetPromptWidget) false false)
      (Audio|PlaySound2D "/Game/Sound/SFX/Distraction.Distraction" 1.0 1.0 0.0 0 0)
      (Utilities|FlowControl|Delay 3.0)
      (Rendering|SetVisibility (Variables|Default|GetPromptWidget) true false)
      (Variables|Default|SetDistractionActive false))))

(event OnBeginCursorOver(ClickCollision)
  (params (TouchedComponent :type Primitive%20Component%20Object%20Reference))
  ;[0 0.9903 1] Hower Over Effects
  (Rendering|SetVisibility (Variables|Default|GetTextRender) true false))

(event OnEndCursorOver(ClickCollision)
  (params (TouchedComponent :type Primitive%20Component%20Object%20Reference))
  ;[0 0.9903 1] Hower Over Effects
  (Rendering|SetVisibility (Variables|Default|GetTextRender) false false))

(event OnComponentBeginOverlap(PromptCollision)
  (params (OverlappedComponent :type Primitive%20Component%20Object%20Reference) (OtherActor :type Actor%20Object%20Reference) (OtherComp :type Primitive%20Component%20Object%20Reference) (OtherBodyIndex :type Integer) (bFromSweep :type Boolean) (SweepResult :type Hit%20Result%20Structure%20%28by%20ref%29))
  ;[0 0.06001 1] Overlapping
  (Utilities|Casting|CastToTopDOwnCharacter_BP OtherActor)
  (Rendering|SetVisibility (Variables|Default|GetTextRender) true false)
  (if (not (Variables|Default|GetDistractionActive))
    (Rendering|SetVisibility (Variables|Default|GetPromptWidget) true false)
    (Variables|Default|SetOverlapping true)
    (Input|EnableInput (Game|GetPlayerController 0))))

(event OnComponentEndOverlap(PromptCollision)
  (params (OverlappedComponent :type Primitive%20Component%20Object%20Reference) (OtherActor :type Actor%20Object%20Reference) (OtherComp :type Primitive%20Component%20Object%20Reference) (OtherBodyIndex :type Integer))
  ;[0 0.06001 1] Overlapping
  (Utilities|Casting|CastToTopDOwnCharacter_BP OtherActor)
  (Rendering|SetVisibility (Variables|Default|GetTextRender) false false)
  (Variables|Default|SetOverlapping false)
  (Input|DisableInput (Game|GetPlayerController 0)))

(event EventBeginPlay
  (bind _returnvalue (Game|GetPlayerController 0))
  ;[1 0.7091 0] Initiate
  (Variables|/Script/Engine.PlayerController|SetbEnableClickEvents _returnvalue true)
  (Variables|/Script/Engine.PlayerController|SetbEnableMouseOverEvents _returnvalue true)
  (Rendering|SetVisibility (Variables|Default|GetPromptWidget) false false))

(event Input|KeyboardEvents|E
  (params (Key :type Key%20Structure :default "None"))
  ;[0 0.2976 1] Triggered
  (:Pressed
    (if (Variables|Default|GetOverlapping)
      (if (Variables|Default|GetDistractionActive)
        (Development|PrintString "Active")
        (else
          (Variables|Default|SetDistractionActive true)
          (Rendering|SetVisibility (Variables|Default|GetPromptWidget) false false)
          (Audio|PlaySound2D "/Game/Sound/SFX/Distraction.Distraction" 1.0 1.0 0.0 0 0)
          (Utilities|FlowControl|Delay 3.0)
          (Rendering|SetVisibility (Variables|Default|GetPromptWidget) true false)
          (Variables|Default|SetDistractionActive false))))))

(fn ConstructionScript)