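; High-voltage box interactable that the player can trigger once to set off a shockwave and explosion.
; Overlapping the top-down character shows the radius, enables input and, while charged, shows the prompt and text; cursor hover reveals radius and text.
; Clicking it, or pressing E in range, activates both effects with sound and spends the charge; later attempts only play a no-charge sound.
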(event OnBeginCursorOver(ClickCollision)
  (params (TouchedComponent :type Primitive%20Component%20Object%20Reference))
  ;[0 0.9903 1] Hower Over Effects
  (Rendering|SetVisibility (Variables|Default|GetRadius) true false)
  (if (Variables|Default|GetCharged)
    (Rendering|SetVisibility (Variables|Default|GetTextRender) true false)))

(event OnClicked(ClickCollision)
  (params (TouchedComponent :type Primitive%20Component%20Object%20Reference) (ButtonPressed :type Key%20Structure))
  ;[0 0.2976 1] Triggered
  (if (Variables|Default|GetCharged)
    (Components|Activation|Activate (Variables|Default|GetSchockwave) false)
    (Audio|PlaySound2D "/Game/Sound/SFX/HVBox_Triggered.HVBox_Triggered" 1.0 1.0 0.0 0 0)
    (Variables|Default|SetCharged false)
    (Rendering|SetVisibility (Variables|Default|Get%20PromptWidget) false false)
    (else
      (Audio|PlaySound2D "/Game/Sound/SFX/HVBox_NoCharge.HVBox_NoCharge" 1.0 1.0 0.0 0 0))))

(event OnEndCursorOver(ClickCollision)
  (params (TouchedComponent :type Primitive%20Component%20Object%20Reference))
  ;[0 0.9903 1] Hower Over Effects
  (Rendering|SetVisibility (Variables|Default|GetTextRender) false false))

(event OnComponentBeginOverlap(PromptCollision)
  (params (OverlappedComponent :type Primitive%20Component%20Object%20Reference) (OtherActor :type Actor%20Object%20Reference) (OtherComp :type Primitive%20Component%20Object%20Reference) (OtherBodyIndex :type Integer) (bFromSweep :type Boolean) (SweepResult :type Hit%20Result%20Structure%20%28by%20ref%29))
  ;[0 0.1884 1] Overlapping
  (Utilities|Casting|CastToTopDOwnCharacter_BP OtherActor)
  (Variables|Default|SetOverlapping true)
  (Rendering|SetVisibility (Variables|Default|GetRadius) true false)
  (Input|EnableInput (Game|GetPlayerController 0))
  (if (Variables|Default|GetCharged)
    (Rendering|SetVisibility (Variables|Default|Get%20PromptWidget) true false)))

(event OnComponentEndOverlap(PromptCollision)
  (params (OverlappedComponent :type Primitive%20Component%20Object%20Reference) (OtherActor :type Actor%20Object%20Reference) (OtherComp :type Primitive%20Component%20Object%20Reference) (OtherBodyIndex :type Integer))
  ;[0 0.1884 1] Overlapping
  (Utilities|Casting|CastToTopDOwnCharacter_BP OtherActor)
  (Rendering|SetVisibility (Variables|Default|Get%20PromptWidget) false false)
  (Variables|Default|SetOverlapping false)
  (Input|DisableInput (Game|GetPlayerController 0)))

(event EventBeginPlay
  (bind _returnvalue (Game|GetPlayerController 0))
  ;[1 0.2687 0.03063] Set Visibility/Useability
  (Variables|/Script/Engine.PlayerController|SetbEnableClickEvents _returnvalue true)
  (Variables|/Script/Engine.PlayerController|SetbEnableMouseOverEvents _returnvalue true)
  (Variables|Default|SetCharged true)
  (Rendering|SetVisibility (Variables|Default|GetTextRender) false false))

(event Input|KeyboardEvents|E
  (params (Key :type Key%20Structure))
  ;[0 0.2976 1] Triggered
  (:Pressed
    (if (Variables|Default|GetOverlapping)
      (if (Variables|Default|GetCharged)
        (Components|Activation|Activate (Variables|Default|GetSchockwave) false)
        (Audio|PlaySound2D "/Game/Sound/SFX/HVBox_Triggered.HVBox_Triggered" 1.0 1.0 0.0 0 0)
        (Variables|Default|SetCharged false)
        (Rendering|SetVisibility (Variables|Default|Get%20PromptWidget) false false)
        (else
          (Audio|PlaySound2D "/Game/Sound/SFX/HVBox_NoCharge.HVBox_NoCharge" 1.0 1.0 0.0 0 0))))))

(fn ConstructionScript)