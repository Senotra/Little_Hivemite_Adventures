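; HVBox_BP is a clickable high-voltage box that sets off its shockwave and explosion components once.
; BeginPlay enables mouse click and hover events on the player controller, sets the box as charged and hides its text and radius indicator.
; Hovering the click collision shows both indicators.
; The first click activates the effects, plays the trigger sound and spends the charge, so later clicks only play a no-charge sound.
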(event OnBeginCursorOver(ClickCollision)
  (params (TouchedComponent :type Primitive%20Component%20Object%20Reference))
  ;[0 0.9903 1] Hower Over Effects
  (Rendering|SetVisibility (Variables|Default|GetTextRender) true false)
  (Rendering|SetVisibility (Variables|Default|GetRadius) true false))

(event OnClicked(ClickCollision)
  (params (TouchedComponent :type Primitive%20Component%20Object%20Reference) (ButtonPressed :type Key%20Structure :default "None"))
  ;[0 0.2976 1] Triggered
  (if (Variables|Default|GetCharged)
    (Components|Activation|Activate (Variables|Default|GetSchockwave) false)
    (Components|Activation|Activate (Variables|Default|GetExplosion) false)
    (Audio|PlaySound2D "/Game/Sound/SFX/HVBox_Triggered.HVBox_Triggered" 1.0 1.0 0.0 0 0)
    (Variables|Default|SetCharged false)
    (else
      (Audio|PlaySound2D "/Game/Sound/SFX/HVBox_NoCharge.HVBox_NoCharge" 1.0 1.0 0.0 0 0))))

(event OnEndCursorOver(ClickCollision)
  (params (TouchedComponent :type Primitive%20Component%20Object%20Reference))
  ;[0 0.9903 1] Hower Over Effects
  (Rendering|SetVisibility (Variables|Default|GetTextRender) false false)
  (Rendering|SetVisibility (Variables|Default|GetRadius) false false))

(event EventBeginPlay
  (bind _returnvalue (Game|GetPlayerController 0))
  ;[1 0.2687 0.03063] Set Visibility/Useability
  (Variables|/Script/Engine.PlayerController|SetbEnableClickEvents _returnvalue true)
  (Variables|/Script/Engine.PlayerController|SetbEnableMouseOverEvents _returnvalue true)
  (Variables|Default|SetCharged true)
  (Rendering|SetVisibility (Variables|Default|GetTextRender) false false)
  (Rendering|SetVisibility (Variables|Default|GetRadius) false false))

(fn ConstructionScript)