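; NPC Blueprint that shows a sequence of dialogue lines and an interaction prompt.
; Interact advances DialogueIndex, lazily creates a Dialogue_Widget to show that Dialogue entry, and removes it once the index exceeds the array length.
; The index increments before the first read and is never reset here.
; PromptTrigger overlaps with TopDOwnCharacter_BP toggle the prompt Widget, which the Construction Script hides initially.
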(event OnComponentBeginOverlap(PromptTrigger)
  (params (OverlappedComponent :type Primitive%20Component%20Object%20Reference) (OtherActor :type Actor%20Object%20Reference) (OtherComp :type Primitive%20Component%20Object%20Reference) (OtherBodyIndex :type Integer) (bFromSweep :type Boolean) (SweepResult :type Hit%20Result%20Structure%20%28by%20ref%29))
  ;[0 0.1261 1] Prompt Visibility
  (Utilities|Casting|CastToTopDOwnCharacter_BP OtherActor)
  (Rendering|SetVisibility (Variables|Default|GetWidget) true false))

(event OnComponentEndOverlap(PromptTrigger)
  (params (OverlappedComponent :type Primitive%20Component%20Object%20Reference) (OtherActor :type Actor%20Object%20Reference) (OtherComp :type Primitive%20Component%20Object%20Reference) (OtherBodyIndex :type Integer))
  ;[0 0.1261 1] Prompt Visibility
  (Utilities|Casting|CastToTopDOwnCharacter_BP OtherActor)
  (Rendering|SetVisibility (Variables|Default|GetWidget) false false))

(event EventInteract
  ;[0.008129 0.1409 1] Dialoge
  (Math|Integer|IncrementInt (Variables|Default|Getdialogue_index)
    (:%20%20
      (if (<= (Variables|Default|Getdialogue_index) (Utilities|Array|Length (Variables|Default|Getdialogue)))
        (Variables|Default|GetUI
          (:then
            _)
          (:else
            (bind _returnvalue (UserInterface|CreateWidget "/Game/Widgets/Dialogue_Widget.Dialogue_Widget_C" (Game|GetPlayerController 0)))
            (bind _output_get (Variables|Default|SetUI _returnvalue))
            (UserInterface|Viewport|AddtoViewport _output_get 0)))
        (Rendering|Components|TextRender|SetText (Variables|/Game/Widgets/Dialogue_Widget.Dialogue_Widget_C|GetDialogueText (Variables|Default|GetUI)) (Utilities|Text|ToText(String) (Utilities|Array|Get(acopy) (Variables|Default|Getdialogue) (Variables|Default|Getdialogue_index))))
        (else
          (bind _output_get_2 (Variables|Default|SetUI (Variables|Default|GetUI)))
          (Widget|RemovefromParent _output_get_2))))))

(fn ConstructionScript
  (Rendering|SetVisibility (Variables|Default|GetWidget) false false))