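; Test NPC Blueprint that walks a looping patrol through the PatrolLocation array, starting on BeginPlay.
; The Patrolling event sets a slow walk speed, calls AIMoveTo, then waits a random few seconds on success before calling itself again.
; The location index increments after that re-call, so each new move reads the previous index, and wraps after four points.
; Failed moves are unhandled, ending the loop.
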(event Custom|Patrolling
  ;[1 1 1] Patrolling
  (Variables|/Script/Engine.CharacterMovementComponent|SetMaxWalkSpeed (Variables|Character|GetCharacterMovement) 1.5e+02)
  (AI|AIMoveTo self (Utilities|Array|Get(acopy) (Variables|Default|GetPatrolLocation) (Variables|Default|GetLocations)) 0 5.0 false
    (:OnSuccess
      (Utilities|FlowControl|Delay (Math|Random|RandomFloatinRange 3.0 6.0))
      (CallFunction|Patrolling)
      (Math|Integer|IncrementInt (Variables|Default|GetLocations)
        (:%20%20
          (if (== (Variables|Default|GetLocations) 4)
            (Variables|Default|SetLocations 0)))))))

(event EventBeginPlay
  ;[0.7816 1 0] Begin
  (CallFunction|Patrolling))

(fn ConstructionScript)