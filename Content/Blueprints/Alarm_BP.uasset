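; Clickable alarm actor that plays a 2D sound and switches its Paper2D flipbook to an on state.
; A click starts the alarm, and a fixed Delay later deactivates the sound and restores the off flipbook.
; Overlap by the top-down character toggles a prompt widget, while cursor hover toggles a text label.
; BeginPlay enables mouse click and hover events on the player controller and hides both prompts.
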(event OnComponentBeginOverlap(PromptTrigger)
  (params (OverlappedComponent :type Primitive%20Component%20Object%20Reference) (OtherActor :type Actor%20Object%20Reference) (OtherComp :type Primitive%20Component%20Object%20Reference) (OtherBodyIndex :type Integer) (bFromSweep :type Boolean) (SweepResult :type Hit%20Result%20Structure%20%28by%20ref%29))
  ;[0 0.09999 1] Prompt Visibility
  (Utilities|Casting|CastToTopDOwnCharacter_BP OtherActor)
  (Rendering|SetVisibility (Variables|Default|GetWidget) true false))

(event OnComponentEndOverlap(PromptTrigger)
  (params (OverlappedComponent :type Primitive%20Component%20Object%20Reference) (OtherActor :type Actor%20Object%20Reference) (OtherComp :type Primitive%20Component%20Object%20Reference) (OtherBodyIndex :type Integer))
  ;[0 0.09999 1] Prompt Visibility
  (Utilities|Casting|CastToTopDOwnCharacter_BP OtherActor)
  (Rendering|SetVisibility (Variables|Default|GetWidget) false false))

(event OnClicked(ClickCollision)
  (params (TouchedComponent :type Primitive%20Component%20Object%20Reference) (ButtonPressed :type Key%20Structure :default "None"))
  ;[0.1676 0.2888 1] Activate / Deactivate Alarm
  (bind _returnvalue (Audio|SpawnSound2D "/Game/Sound/SFX/Alarm.Alarm" 1.0 1.0 0.0 0))
  (Components|Activation|SetActive _returnvalue true false)
  (Sprite|SetFlipbook (Variables|Default|GetAlarm) "/Game/LevelPrototyping/Textures/scifi_items2_alternated_sprites/AlarmOn_FB.AlarmOn_FB")
  (Utilities|FlowControl|Delay 2e+01)
  (Components|Activation|SetActive _returnvalue false false)
  (Sprite|SetFlipbook (Variables|Default|GetAlarm) "/Game/LevelPrototyping/Textures/scifi_items2_alternated_sprites/AlarmOff_FB.AlarmOff_FB"))

(event OnBeginCursorOver(ClickCollision)
  (params (TouchedComponent :type Primitive%20Component%20Object%20Reference))
  ;[0 0.6669 1] Comment
  (Rendering|SetVisibility (Variables|Default|GetTextRender) true false))

(event OnEndCursorOver(ClickCollision)
  (params (TouchedComponent :type Primitive%20Component%20Object%20Reference))
  ;[0 0.6669 1] Comment
  (Rendering|SetVisibility (Variables|Default|GetTextRender) false false))

(event EventBeginPlay
  (bind _returnvalue (Game|GetPlayerController 0))
  ;[1 1 1] Comment
  (Variables|/Script/Engine.PlayerController|SetbEnableClickEvents _returnvalue true)
  (Variables|/Script/Engine.PlayerController|SetbEnableMouseOverEvents _returnvalue true)
  (Rendering|SetVisibility (Variables|Default|GetWidget) false false)
  (Rendering|SetVisibility (Variables|Default|GetTextRender) false false))

(fn ConstructionScript)